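; AIC_Runner is an AI controller that drives a BP_Runner pawn by faking alternating left and right power inputs.
; On possess it caches the runner.
; A one-shot timer, re-armed after each input with a random delay between MinInputDelay and MaxInputDelay, paces the presses, and a FlipFlop alternates the side for an irregular input rhythm.
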(event `self.ReceiveBeginPlay`
  (`KismetSystemLibrary.K2_SetTimerDelegate` (`|CreateDelegate` :!event `SimulateInput`) (`KismetMathLibrary.RandomFloatInRange` (`self.MinInputDelay`) (`self.MaxInputDelay`)) :!label _label))

(event `self.ReceivePossess`
  (params (PossessedPawn :type "Pawn Object Reference"))
  (bind _asbp_runner (cast `/Game/Blueprints/BP_Runner` PossessedPawn))
  (set `self.OwnedRunner` _asbp_runner))

(event `SimulateInput`
  (`/Engine/EditorBlueprintResources/StandardMacros.FlipFlop`
    (:`A`
      (`/Game/Blueprints/BP_Runner.SimulatePowerLeft` (`self.OwnedRunner`))
      (goto _label))
    (:`B`
      (`/Game/Blueprints/BP_Runner.SimulatePowerRight` (`self.OwnedRunner`))
      (goto _label))))

(fn `UserConstructionScript`)